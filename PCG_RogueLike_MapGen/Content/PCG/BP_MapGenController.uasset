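; Map generation controller that fills the bounds of its Cube with randomly chosen terrain chunks on a 3D grid at BeginPlay.
; It builds positions layer by layer from the bottom up, then selects and spawns a node-sized chunk at each.
; Downward traces check whether the chunk below allows spawning above it, gating underground chunks under a height cap and topper chunks.
; A height-based weighting sets the odds of a topper over an underground chunk.
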(event EventBeginPlay
  (bind _nodesize (Variables|Default|GetNodeSize))
  ;[0 0 0 0.5] Set Vectors For Spawn Parameters
  (bind _output_get (Variables|Default|SetRelativeGeneratorBounds (- (* (Transformation|GetWorldScale (Variables|Default|GetCube)) 5e+01) (* (Variables|Default|GetNodeSize) 5e+01))))
  (Variables|Default|SetWorldGeneratorBounds (+ _output_get (Transformation|GetWorldLocation (Variables|Default|GetCube))))
  (bind _output_get_2 (Variables|Default|SetSpawnPosTemp (+ (Transformation|GetWorldLocation (Variables|Default|GetCube)) (* (Variables|Default|GetRelativeGeneratorBounds) -1.0))))
  (Utilities|Array|AddUnique (Variables|Default|GetChunkSpawnPos) _output_get_2)
  ;[0 0 0 0.5] Loop To Add Vectors To Array
  (while (not (> (.z (Variables|Default|GetSpawnPosTemp)) (.z (Variables|Default|GetWorldGeneratorBounds))))
    (while (not (> (.x (Variables|Default|GetSpawnPosTemp)) (.x (Variables|Default|GetWorldGeneratorBounds))))
      (while (!= (.y (Variables|Default|GetSpawnPosTemp)) (.y (Variables|Default|GetWorldGeneratorBounds)))
        (bind _output_get_3 (Variables|Default|SetSpawnPosTemp (Math|Vector|MakeVector (.x (Variables|Default|GetSpawnPosTemp)) (+ (.y (Variables|Default|GetSpawnPosTemp)) (* (Variables|Default|GetNodeSize) 1e+02)) (.z (Variables|Default|GetSpawnPosTemp)))))
        (Utilities|Array|AddUnique (Variables|Default|GetChunkSpawnPos) _output_get_3))
      (Variables|Default|SetSpawnPosTemp (Math|Vector|MakeVector (+ (.x (Variables|Default|GetSpawnPosTemp)) (* (Variables|Default|GetNodeSize) 1e+02)) (- (+ (.y (Transformation|GetWorldLocation (Variables|Default|GetCube))) (* (.y (Variables|Default|GetRelativeGeneratorBounds)) -1.0)) (* (Variables|Default|GetNodeSize) 1e+02)) (.z (Variables|Default|GetSpawnPosTemp)))))
    (Variables|Default|SetSpawnPosTemp (Math|Vector|MakeVector (+ (.x (Transformation|GetWorldLocation (Variables|Default|GetCube))) (* (.x (Variables|Default|GetRelativeGeneratorBounds)) -1.0)) (.y (Variables|Default|GetSpawnPosTemp)) (+ (.z (Variables|Default|GetSpawnPosTemp)) (* (Variables|Default|GetNodeSize) 1e+02)))))
  ;[0 0 0 0.5] Run Through Array, Select Chunk, Spawn Chunk
  (for _array_element (Variables|Default|GetChunkSpawnPos)
    (bind _selectedchunk (CallFunction|SelectNodeType _array_element))
    (Game|SpawnActorfromClass _selectedchunk (Math|Transform|MakeTransform _array_element "0, 0, 0" (Math|Vector|MakeVector _nodesize _nodesize _nodesize)) "Undefined" "MultiplyWithRoot" 0 0)))

(event EventDebug
  ;[0 0 0 0.5] Debug
  (Development|PrintString (Utilities|String|ToString(Vector) (Variables|Default|GetRelativeGeneratorBounds)) true true "(R=0.000000,G=0.660000,B=1.000000,A=1.000000)" 1e+14))

(fn ConstructionScript)

(fn SelectNodeType
  (params (NodeToChange :type Vector))
  (ChunkSpawnConditions|CanUndergroundSpawn NodeToChange)
  (ChunkSpawnConditions|CanTopperSpawn NodeToChange)
  (bind _selectedchunk (CallFunction|RandomSelect))
  (CallFunction|VariableReset)
  (return _selectedchunk))

(fn RandomSelect
  (bind _topperchunkarray (Variables|Chunks|GetTopperChunkArray))
  (bind _undergroundchunkarray (Variables|Chunks|GetUndergroundChunkArray))
  (bind _spawntop (CallFunction|WeightCalculator))
  (if _spawntop
    (bind _result (Math|Integer|DecrementInt (Utilities|Array|Length _topperchunkarray))
      (:%20%20
        (return (Utilities|Array|Get(acopy) _topperchunkarray (Math|Random|RandomIntegerinRange 0 _result)))))
    (elif (Variables|Default|GetSpawnUnderground)
      (bind _result_2 (Math|Integer|DecrementInt (Utilities|Array|Length _undergroundchunkarray))
        (:%20%20
          (return (Utilities|Array|Get(acopy) _undergroundchunkarray (Math|Random|RandomIntegerinRange 0 _result_2))))))))

(fn CanUndergroundSpawn
  (params (NodeToChange :type Vector))
  (if (not (>= (- (.z NodeToChange) (.z (Transformation|GetWorldLocation (Variables|Default|GetCube)))) 1e+04))
    (bind _outhit (Collision|LineTraceByChannel (Math|Vector|MakeVector (.x NodeToChange) (.y NodeToChange) (.z NodeToChange)) (Math|Vector|MakeVector (.x NodeToChange) (.y NodeToChange) (- (.z NodeToChange) (* (.z (Transformation|GetWorldScale (Variables|Default|GetCube))) 1e+02))) "TraceTypeQuery1" false 0 "None"))
    (if (not (== (.HitActor (Collision|BreakHitResult _outhit)) 0))
      (bind _canspawnabove_ (Class|BPIMapNode|GetSpawnAbove(Message) (.HitActor (Collision|BreakHitResult _outhit))))
      (if _canspawnabove_
        (Variables|Default|SetSpawnUnderground true :!label _label))
      (else
        (goto _label)))))

(fn CanTopperSpawn
  (params (NodeToChange :type Vector))
  (bind _outhit (Collision|LineTraceByChannel (Math|Vector|MakeVector (.x NodeToChange) (.y NodeToChange) (.z NodeToChange)) (Math|Vector|MakeVector (.x NodeToChange) (.y NodeToChange) (- (.z NodeToChange) (* (.z (Transformation|GetWorldScale (Variables|Default|GetCube))) 1e+02))) "TraceTypeQuery1" false 0 "None"))
  (if (not (== (.HitActor (Collision|BreakHitResult _outhit)) 0))
    (bind _canspawnabove_ (Class|BPIMapNode|GetSpawnAbove(Message) (.HitActor (Collision|BreakHitResult _outhit))))
    (else
      (bind _output_get (Variables|Default|SetCanSpawnAbove? true))))
  (if (or _canspawnabove_ _output_get)
    (Variables|Default|SetTopperWeighting (Utilities|Select :Index (/ (Math|Float|Truncate (+ (- (.z NodeToChange) (.z (Transformation|GetWorldLocation (Variables|Default|GetCube)))) (* (.z (Transformation|GetWorldScale (Variables|Default|GetCube))) 5e+01))) 5000) :Option%200 25 :Option%201 25 :Option%202 50 :Option%203 70 :Option%204 100))))

(fn WeightCalculator
  (return (>= (Math|Random|RandomFloatinRange 0.0 1e+02) (- 1e+02 (Variables|Default|GetTopperWeighting)))))

(fn VariableReset
  (Variables|Default|SetSpawnUnderground false)
  (Variables|Default|SetTopperWeighting 0)
  (Variables|Default|SetCanSpawnAbove? false))